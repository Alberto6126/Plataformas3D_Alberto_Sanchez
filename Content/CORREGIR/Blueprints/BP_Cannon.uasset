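; BP_Cannon is a cannon that automatically fires projectiles at a regular interval for as long as it runs.
; BeginPlay starts the CannonTimer macro, an endless Delay loop that waits for the cadence before each SpawnProjectile call.
; SpawnProjectile spawns at the Spawner's world location, ignoring its rotation, then passes speed and shot direction (Sense) to the projectile and sets its lifespan.
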(event EventBeginPlay
  (Utilities|CannonTimer))

(event Collision|EventActorBeginOverlap
  (params (OtherActor :type Actor%20Object%20Reference)))

(event EventTick
  (params (DeltaSeconds :type Float%20%28single-precision%29)))

(fn ConstructionScript)

(fn SpawnProjectile
  (bind _returnvalue (Game|SpawnActorfromClass "/Game/CORREGIR/Blueprints/Projectile.Projectile_C" (Math|Conversions|ToTransform(Vector) (Transformation|GetWorldLocation (Variables|Default|GetSpawner))) "Undefined" "MultiplyWithRoot" 0 0))
  (Variables|/Game/CORREGIR/Blueprints/Projectile.Projectile_C|SetSpeed _returnvalue (Variables|Default|GetProjectileSpeed))
  (Variables|/Game/CORREGIR/Blueprints/Projectile.Projectile_C|SetSense _returnvalue (Variables|Default|GetShootSense))
  (Actor|SetLifeSpan _returnvalue (Variables|Default|GetProjectileLifespan))
  (return))