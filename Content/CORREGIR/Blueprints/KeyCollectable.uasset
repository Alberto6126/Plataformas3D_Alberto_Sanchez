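; KeyCollectable is a key pickup that spins in place and is collected when a BP_ThirdPersonCharacter overlaps it.
; On BeginPlay it caches the level's GameManager, then each Tick rotates its root around yaw by RotationSpeed and RotationSense.
; Collection marks its ID active on the GameManager, calls KeyCollected, then hides the mesh and disables box collision instead of destroying the actor.
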(event EventBeginPlay
  (CallFunction|GetGameManager))

(event Collision|EventActorBeginOverlap
  (params (OtherActor :type Actor%20Object%20Reference))
  (Utilities|Casting|CastToBP_ThirdPersonCharacter OtherActor)
  (Utilities|CollectKey))

(event EventTick
  (params (DeltaSeconds :type Float%20%28single-precision%29))
  (Utilities|ObjectRotation DeltaSeconds))

(fn ConstructionScript)

(fn GetGameManager
  (bind _returnvalue (Actor|GetActorOfClass "/Game/CORREGIR/Blueprints/GameManager.GameManager_C"))
  (Variables|Default|SetGameManagerRef _returnvalue))