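; BP_CollectableJetpack is a pickup actor that grants the jetpack to the player character.
; On overlap with a BP_ThirdPersonCharacter, it calls SetJetpackOn on the character and hides its own Jetpack component rather than destroying the actor.
; Every tick, ObjectRotation spins the actor around its local yaw axis, scaled by delta time, speed and direction variables.
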(event Collision|EventActorBeginOverlap
  (params (OtherActor :type Actor%20Object%20Reference))
  ;[1 1 1] Si el actor con el que colisiona es el personaje, se activa el Jetpack tanto lógicamente como visualmente
  (bind _asbp_third_person_character (Utilities|Casting|CastToBP_ThirdPersonCharacter OtherActor))
  (Default|SetJetpackon _asbp_third_person_character)
  (Rendering|SetVisibility (Variables|Default|GetJetpack) false false))

(event EventTick
  (params (DeltaSeconds :type Float%20%28single-precision%29))
  (Utilities|ObjectRotation DeltaSeconds))

(fn ConstructionScript)