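; Game manager that runs the timed two-key puzzle, tracks total play time and handles end-of-game restart.
; Collecting a key resets a countdown; a Delay-based loop checks both keys each second, opening FinalDoor on success or restoring the keys on timeout.
; BeginPlay stores the first found Checkpoint's location, and Tick accumulates game time.
; FinalPrint shows that time, then triggers a countdown that reloads ThirdPersonMap.
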(event Custom|KeyCollected
  ;[1 1 1] Al conseguir una llave, se setea el countdown al máximo y se comprueba si ambas ya han sido recolectadas, en el caso de se avisa de que se ha abierto una puerta, en el caso de no recolectarlas todas, se reinician
  (Variables|Default|SetKeyTimer (Variables|Default|GetCountdownKeyValue))
  (bind _haswon (CallFunction|CheckKeys))
  (if (not _haswon)
    (Development|PrintString "INICIANDO CUENTA ATRÁS")
    (Utilities|KeyTimerController
      (:CollectedAll
        (Utilities|HandleKeyEnded :!label _label))
      (:Missed
        (goto _label Failed)))))

(event Custom|onGameEnded
  ;[1 1 1] Al acabar la partida se imprime una string en bucle con el tiempo que falta hasta reiniciar, y luego se recarga el nivel
  (Development|PrintString "REINICIANDO PARTIDA EN: ...")
  (Utilities|GameEndedTimer
    (:Out
      (Game|OpenLevel(byObjectReference) "/Game/ThirdPerson/Maps/ThirdPersonMap.ThirdPersonMap"))))

(event EventBeginPlay
  (Utilities|CheckPointManagement))

(event EventTick
  (params (DeltaSeconds :type Float%20%28single-precision%29))
  ;[1 1 1] Timer para controlar lo que tarda el jugador en pasarse el juego
  (Utilities|GameTimerManager DeltaSeconds))

(fn ConstructionScript)

(fn SetKeyActive
  (params (keyID :type Integer))
  ;[1 1 1] Se revisa que todas las keys con ID diferentes estén recogidas, en el caso de recoger una key con una ID no contemplada, se alerta de un error
  (switch int keyID
    (:Default
      (Development|PrintString "Key no registrada" true true "(R=1.000000,G=0.000000,B=0.006919,A=1.000000)"))
    (:0
      (Variables|Default|SetKey_1 true))
    (:1
      (Variables|Default|SetKey_2 true))))

(fn FinalPrint
  ;[1 1 1] Se imprime el tiempo total de juego hasta que el jugador se ha pasado el juego, luego se llama al evento onGameEnded
  (Development|PrintString (Utilities|String|Append (Utilities|String|Append "Has conseguido llegar a casa en: " (Utilities|String|ToString(Integer) (Math|Float|Truncate (Variables|Default|GetGameTimer)))) " segundos, enhorabuena!") true true "(R=0.060520,G=1.000000,B=0.000000,A=1.000000)" 1e+01)
  (CallFunction|OnGameEnded))

(fn CheckKeys
  (return (and (Variables|Default|GetKey_1) (Variables|Default|GetKey_2))))

(fn OpenDoor
  (bind _returnvalue (Actor|GetActorOfClass "/Game/CORREGIR/Blueprints/FinalDoor.FinalDoor_C"))
  (Default|OpenDoor _returnvalue))

(fn RestartKeys
  ;[1 1 1] Se resetean las llaves tanto lógica como visualmente
  (Variables|Default|SetKey_1 false)
  (Variables|Default|SetKey_2 false)
  (bind _outactors (Actor|GetAllActorsOfClass "/Game/CORREGIR/Blueprints/KeyCollectable.KeyCollectable_C"))
  (for _array_element _outactors
    (Rendering|SetVisibility (Variables|/Game/CORREGIR/Blueprints/KeyCollectable.KeyCollectable_C|GetStaticMesh _array_element) true false)
    (Collision|SetCollisionEnabled (Variables|/Game/CORREGIR/Blueprints/KeyCollectable.KeyCollectable_C|GetBox _array_element) "QueryAndPhysics")))